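; Interactive object actor that, when used, tweens the calling actor to its InteractionLocation on X and Y, keeping the caller's height.
; On BeginPlay it rebinds the BasicInteraction component's PreExecution, Execution and PostExecution events to its own handlers.
; The handlers chain manually: pre-execution fires execution, which runs the TweenLocation move and then fires post-execution to run PostExecutionSetup.
; Debug prints mark each stage.
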(event `self.ReceiveBeginPlay`
  (bind _basicinteraction (`self.BasicInteraction`))
  (`parent.ReceiveBeginPlay`)
  (clear `BasicInteractionComponent.OnPreExecution` _basicinteraction)
  (clear `BasicInteractionComponent.OnExecution` _basicinteraction)
  (clear `BasicInteractionComponent.OnPostExecution` _basicinteraction)
  (add `BasicInteractionComponent.OnPreExecution` _basicinteraction (delegate `PreExecution`))
  (add `BasicInteractionComponent.OnExecution` _basicinteraction (delegate `Execution`))
  (add `BasicInteractionComponent.OnPostExecution` _basicinteraction (delegate `PostExecution`)))

(event `PreExecution`
  (params (caller :type "Object Object Reference") (component :type "ActorComponent Object Reference") (interactionType :type "EBasicInteractionType Enum" :default "DEFAULT"))
  (`BasicInteractionComponent.OnExecution` (`self.BasicInteraction`) caller component interactionType)
  (`KismetSystemLibrary.PrintString` "PreExecution!!!1"))

(event `Execution`
  (params (caller :type "Object Object Reference") (component :type "ActorComponent Object Reference") (interactionType :type "EBasicInteractionType Enum" :default "DEFAULT"))
  (bind _asactor (cast `Actor` caller))
  (bind _returnvalue (`self.K2_GetActorLocation` _asactor))
  (`TweenFunctionLibrary.TweenLocation` _asactor _returnvalue (`KismetMathLibrary.MakeVector` (.x (`SceneComponent.K2_GetComponentLocation` (`self.InteractionLocation`))) (.y (`SceneComponent.K2_GetComponentLocation` (`self.InteractionLocation`))) (.z _returnvalue)))
  (`KismetSystemLibrary.PrintString` "TweenCompleted" true true (struct :`R` 1.0 :`B` 0.030305 :`A` 1.0))
  (`BasicInteractionComponent.OnPostExecution` (`self.BasicInteraction`) caller component interactionType))

(event `PostExecution`
  (params (caller :type "Object Object Reference") (component :type "ActorComponent Object Reference") (interactionType :type "EBasicInteractionType Enum" :default "DEFAULT"))
  (`BasicInteractionComponent.PostExecutionSetup` (`self.BasicInteraction`) interactionType)
  (`KismetSystemLibrary.PrintString` "PostExecution"))

(fn `UserConstructionScript`
  (`parent.UserConstructionScript`))