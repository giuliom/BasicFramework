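; BP_InteractiveTween is an interactable actor that tweens its own rotation when its BasicInteraction event executes.
; OnExecution calls TweenRotation on the actor with a 180-degree single-axis target over two seconds.
; An ExecutionInProgress flag wraps the tween as a guard against re-triggering while it is set.
; BeginPlay, overlap and Tick are disabled stubs, so all behavior comes from the interaction event.
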(event `self.BasicInteraction.OnExecution`
  (params (caller :type "Object Object Reference") (component :type "ActorComponent Object Reference") (interactionType :type "BasicInteractionType Object Reference"))
  (if (not (`self.executionInProgress`))
    (set `self.executionInProgress` true)
    (`TweenFunctionLibrary.TweenRotation` self (struct) (struct :`Yaw` 180.0) "LINEAR" 2.0)
    (set `self.executionInProgress` false)))

(fn `UserConstructionScript`
  (`parent.UserConstructionScript`))