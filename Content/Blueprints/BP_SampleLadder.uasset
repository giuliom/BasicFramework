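; BP_SampleLadder is a sample ladder that characters enter through a BasicInteraction.
; On execution, it tweens the caller to InteractionLocation's horizontal position while keeping the caller's height.
; It then sets the BasicCharacterMovementComponent's custom mode to LADDER, with the base movement mode passed as None.
; Debug prints mark each interaction phase; climbing logic is not in this Blueprint.
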(event `self.ReceiveBeginPlay`)

(event `self.BasicInteraction.OnPreExecution`
  (params (caller :type "Object Object Reference") (component :type "ActorComponent Object Reference") (interactionType :type Byte))
  (`KismetSystemLibrary.PrintString` "PreExecution!!!1"))

(event `self.BasicInteraction.OnExecution`
  (params (caller :type "Object Object Reference") (component :type "ActorComponent Object Reference") (interactionType :type Byte))
  (bind _asactor (cast `Actor` caller))
  (bind _returnvalue (`self.K2_GetActorLocation` _asactor))
  (`TweenFunctionLibrary.TweenLocation` _asactor _returnvalue (`KismetMathLibrary.MakeVector` (.x (`SceneComponent.K2_GetComponentLocation` (`self.InteractionLocation`))) (.y (`SceneComponent.K2_GetComponentLocation` (`self.InteractionLocation`))) (.z _returnvalue)))
  (`KismetSystemLibrary.PrintString` "TweenCompleted" true true (struct :`R` 1.0 :`B` 0.030305 :`A` 1.0))
  (bind _asbasic_character (cast `BasicCharacter` caller))
  (bind _asbasic_character_movement_component (cast `BasicCharacterMovementComponent` (`Pawn.GetMovementComponent` _asbasic_character)))
  (`CharacterMovementComponent.SetMovementMode` _asbasic_character_movement_component "MOVE_None" (enumliteral `EBasicCharacterCustomMovementMode` "CMOVE_LADDER")))

(event `self.BasicInteraction.OnPostExecution`
  (params (caller :type "Object Object Reference") (component :type "ActorComponent Object Reference") (interactionType :type Byte))
  (`KismetSystemLibrary.PrintString` "PostExecution"))

(fn `UserConstructionScript`
  (`parent.UserConstructionScript`))